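; RTS camera controller that moves, rotates and zooms the player's CameraPawn.
; Axis input moves the pawn along its local axes at a speed scaled by spring arm length, and screen-edge mouse checks add local offsets.
; Holding Pan opens gates for mouse yaw and clamped pitch while suspending movement; PanReset levels pitch.
; Zoom inputs adjust the spring arm length within limits.
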(event EventBeginPlay
  ;[1 1 1] Set Ref
  (Utilities|FlowControl|Sequence
    (:then_0
      (Utilities|ReferenceCasts))))

(event Input|ActionEvents|InputActionZoomIn
  (params (Key :type Key%20Structure :default "AnyKey"))
  (bind _camerapawnref (Variables|Reference|GetCameraPawnRef))
  (bind _springarm (Variables|/Game/FirstRTS/Blueprints/CameraPawn.CameraPawn_C|GetSpringArm _camerapawnref))
  ;[1 1 1] Zoom In/Out
  (:Pressed
    (Variables|/Script/Engine.SpringArmComponent|SetTargetArmLength _springarm (Math|Float|Clamp(Float) (- (Variables|/Script/Engine.SpringArmComponent|GetTargetArmLength _springarm) (Variables|Default|GetZoomSensetivity)) 5e+02 (Variables|Default|GetMaxArmDistance)))))

(event Input|ActionEvents|InputActionZoomOut
  (params (Key :type Key%20Structure :default "AnyKey"))
  (bind _camerapawnref (Variables|Reference|GetCameraPawnRef))
  (bind _springarm (Variables|/Game/FirstRTS/Blueprints/CameraPawn.CameraPawn_C|GetSpringArm _camerapawnref))
  ;[1 1 1] Zoom In/Out
  (:Pressed
    (Variables|/Script/Engine.SpringArmComponent|SetTargetArmLength _springarm (Math|Float|Clamp(Float) (+ (Variables|Default|GetZoomSensetivity) (Variables|/Script/Engine.SpringArmComponent|GetTargetArmLength _springarm)) 5e+02 (Variables|Default|GetMaxArmDistance)))))

(event Input|ActionEvents|InputActionPan
  (params (Key :type Key%20Structure :default "AnyKey"))
  (bind _camerapawnref (Variables|Reference|GetCameraPawnRef))
  (bind _returnvalue (Transformation|GetActorRotation _camerapawnref))
  (bind (_roll _pitch _yaw) (Math|Rotator|BreakRotator _returnvalue))
  ;[1 1 1] PanX
  (:Pressed
    (Variables|Default|SetDisableCamNav true)
    (Utilities|FlowControl|Gate true) ; enters at Open
  )
  (:Released
    (Variables|Default|SetDisableCamNav false)
    (Utilities|FlowControl|Gate true) ; enters at Close
  ))

(event Input|ActionEvents|InputActionPan
  (params (Key :type Key%20Structure :default "AnyKey"))
  (bind _camerapawnref (Variables|Reference|GetCameraPawnRef))
  (bind _returnvalue (Transformation|GetActorRotation _camerapawnref))
  (bind (_roll _pitch _yaw) (Math|Rotator|BreakRotator _returnvalue))
  ;[1 1 1] PanY
  (:Pressed
    (Variables|Default|SetDisableCamNav true)
    (Utilities|FlowControl|Gate true) ; enters at Open
  )
  (:Released
    (Variables|Default|SetDisableCamNav false)
    (Utilities|FlowControl|Gate true) ; enters at Close
  ))

(event Input|ActionEvents|InputActionPanReset
  (params (Key :type Key%20Structure :default "AnyKey"))
  (bind _returnvalue (Transformation|GetActorRotation))
  (bind (_roll _pitch _yaw) (Math|Rotator|BreakRotator _returnvalue))
  ;[1 1 1] PanReset
  (:Pressed
    (Transformation|SetActorRotation (Variables|Reference|GetCameraPawnRef) (Math|Rotator|MakeRotator _roll 0.0 _yaw))))

(event Input|AxisEvents|InputAxisMoveForward
  (params (AxisValue :type Float%20%28single-precision%29))
  ;[1 1 1] Movement X
  (if (not (Variables|Default|GetDisableCamNav))
    (Transformation|SetActorTransform (Variables|Reference|GetCameraPawnRef) (Utilities|MovementX AxisValue (CallFunction|MovementSpeedCalculation) (Variables|Default|GetFastMoveMultiplier) (Variables|Reference|GetCameraPawnRef)))))

(event Input|AxisEvents|InputAxisMoveRight
  (params (AxisValue :type Float%20%28single-precision%29))
  (bind _movesensitivity (CallFunction|MovementSpeedCalculation))
  (bind _fastmovemultiplier (Variables|Default|GetFastMoveMultiplier))
  (bind _camerapawnref (Variables|Reference|GetCameraPawnRef))
  (bind _transform (Utilities|MovementY AxisValue _movesensitivity _fastmovemultiplier _camerapawnref))
  (bind (_location _rotation _scale) (Math|Transform|BreakTransform _transform))
  (bind (_x _y) (Math|Vector|BreakVector _location))
  ;[1 1 1] Movement Y
  (if (not (Variables|Default|GetDisableCamNav))
    (Transformation|SetActorTransform (Variables|Reference|GetCameraPawnRef) (Math|Transform|MakeTransform (Math|Vector|MakeVector _x _y 1e+02) _rotation _scale))))

(event Input|MouseEvents|MouseX
  (params (AxisValue :type Float%20%28single-precision%29))
  (bind _camerapawnref (Variables|Reference|GetCameraPawnRef))
  (bind _returnvalue (Transformation|GetActorRotation _camerapawnref))
  (bind (_roll _pitch _yaw) (Math|Rotator|BreakRotator _returnvalue))
  ;[1 1 1] PanX
  (Utilities|FlowControl|Gate true
    (:Exit
      (Transformation|SetActorRotation (Variables|Reference|GetCameraPawnRef) (Math|Rotator|MakeRotator _roll _pitch (+ (* (Variables|Default|GetPanSensitivity) AxisValue) _yaw))))))

(event Input|MouseEvents|MouseY
  (params (AxisValue :type Float%20%28single-precision%29))
  (bind _camerapawnref (Variables|Reference|GetCameraPawnRef))
  (bind _returnvalue (Transformation|GetActorRotation _camerapawnref))
  (bind (_roll _pitch _yaw) (Math|Rotator|BreakRotator _returnvalue))
  ;[1 1 1] PanY
  (Utilities|FlowControl|Gate true
    (:Exit
      (Transformation|SetActorRotation (Variables|Reference|GetCameraPawnRef) (Math|Rotator|MakeRotator _roll (Math|Float|Clamp(Float) (+ (* (Variables|Default|GetPanSensitivity) AxisValue) _pitch) -15.0 45.0) _yaw)))))

(event Input|MouseEvents|MouseX
  (params (AxisValue :type Float%20%28single-precision%29))
  ;[1 1 1] Edge Movements
  (if (not (Variables|Default|GetDisableCamNav))
    (bind (_delta_xspeed _delta_yspeed) (Utilities|ScreenEdgeMovement))
    (Transformation|AddActorLocalOffset (Variables|Reference|GetCameraPawnRef) (Math|Vector|MakeVector _delta_xspeed _delta_yspeed 0.0) true false)))

(event Input|MouseEvents|MouseY
  (params (AxisValue :type Float%20%28single-precision%29))
  ;[1 1 1] Edge Movements
  (if (not (Variables|Default|GetDisableCamNav))
    (Utilities|ScreenEdgeMovement) ; enters at MouseY
  ))

(fn ConstructionScript)

(fn MovementSpeedCalculation
  (return (Math|Float|Clamp(Float) (/ (Variables|/Script/Engine.SpringArmComponent|GetTargetArmLength (Variables|/Game/FirstRTS/Blueprints/CameraPawn.CameraPawn_C|GetSpringArm (Variables|Reference|GetCameraPawnRef))) 1e+02) 5.0 2e+01)))